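; Player controller that shows the introduction widget on BeginPlay and manages the pause menu.
; IA_Pause and the HandlePauseSystem event share one toggle, which is blocked once GameOver is set.
; The stored menu reference acts as the pause state, with the toggle creating or removing the main menu widget while switching game pause, input mode and cursor visibility.
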(event `self.ReceiveBeginPlay`
  (bind _returnvalue (`|CreateWidget` "/Game/-Blueprints/Widgets/WBP_Introduction.WBP_Introduction_C"))
  (`UserWidget.AddToViewport` _returnvalue 0))

(event `HandlePauseSystem`
  (bind _returnvalue (`GameplayStatics.GetPlayerController` 0))
  (bind _returnvalue_2 (`GameplayStatics.GetPlayerController` 0))
  ;[1 0.8363 0 0.5] Pause System
  ;;[1 0.8363 0 0.5] Check game over for pause accessibility.
  (if (not (`self.GameOver`)) :!label _label
    ;;[1 0.8363 0 0.5] Check if pause is active or not to act accordingly.
    (`/Engine/EditorBlueprintResources/StandardMacros.IsValid` (`self.MenuRef`)
      (:`Is Valid`
        (`GameplayStatics.SetGamePaused` false)
        ;;[1 0.8363 0 0.5] Remove/Add menu widget... Set input modes... Set mouse visibility... Remove menu reference if pause is being disabled.
        (`Widget.RemoveFromParent` (`self.MenuRef`))
        (`WidgetBlueprintLibrary.SetInputMode_GameOnly` _returnvalue)
        (set `PlayerController.bShowMouseCursor` false _returnvalue)
        (set `self.MenuRef` null))
      (:`Is Not Valid`
        (`GameplayStatics.SetGamePaused` true)
        (bind _returnvalue_3 (`|CreateWidget` "/Game/-Blueprints/Widgets/WBP_MainMenu.WBP_MainMenu_C"))
        (bind _output_get (set `self.MenuRef` _returnvalue_3))
        (`UserWidget.AddToViewport` _output_get 0)
        (`WidgetBlueprintLibrary.SetInputMode_GameAndUIEx` _returnvalue_2 null)
        (set `PlayerController.bShowMouseCursor` true _returnvalue_2)))))

(event `EnhancedInput|/Game/-Blueprints/Character/Inputs/Actions/IA_Pause`
  (params (ActionValue :type Boolean) (ElapsedSeconds :type "Float (double-precision)") (TriggeredSeconds :type "Float (double-precision)") (InputAction :type "InputAction Object Reference" :default "/Game/-Blueprints/Character/Inputs/Actions/IA_Pause.IA_Pause"))
  ;[1 0.8363 0 0.5] Pause System
  (:`Started`
    (goto _label)))

(fn `UserConstructionScript`)