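; BP_CombatNPC1 is a combat NPC Blueprint meant to chase the player.
; BeginPlay and Tick call MoveTowardsPlayer, and Tick also calls GetPlayerPosition, but both are empty stubs.
; The chase logic sits in two custom events with no caller here.
; One casts the player character to BP_LucidDriver and issues AIMoveTo toward it; the other stores the player's location as PlayerPOS.
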(event `self.ReceiveBeginPlay`
  (`self.Move Towards Player`))

(event `self.ReceiveTick`
  (params (DeltaSeconds :type "Float (single-precision)"))
  (`self.Get Player Position`)
  (`self.Move Towards Player`))

(event `CustomEvent`
  (bind _asbp_lucid_driver (cast `/Game/-Blueprints/Character/BP_LucidDriver` (`GameplayStatics.GetPlayerCharacter` 0)))
  (bind _output_get (set `self.Player Ref` _asbp_lucid_driver))
  (`|AIMoveTo` self (`self.Player POS`) _output_get))

(event `CustomEvent_1`
  (set `self.Player POS` (`self.K2_GetActorLocation` (`self.Player Ref`))))

(event `Move Towards Player`)

(fn `Get Player Position`)

(fn `UserConstructionScript`)