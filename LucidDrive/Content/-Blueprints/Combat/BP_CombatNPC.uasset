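; BP_CombatNPC is an enemy character that chases the player's BP_LucidDriver and attacks it in melee range.
; Tick caches the player's location and reissues AIMoveTo every frame.
; Overlapping the AttackRange component stops movement and sets IsInRange, which is never cleared as end overlap is empty.
; While IsInRange is set, each Tick plays a random montage from AttackMontages, with no cooldown.
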(event `self.ReceiveBeginPlay`
  (`self.Move Towards Player`))

(event `self.ReceiveTick`
  (params (DeltaSeconds :type "Float (single-precision)"))
  (`self.Get Player Position`)
  (if (stale `self.AttackRange.OnComponentBeginOverlap` _output_get)
    (`self.PerformAttack`))
  (`self.Move Towards Player`))

(event `Move Towards Player`
  (bind _asbp_lucid_driver (cast `/Game/-Blueprints/Character/BP_LucidDriver` (`GameplayStatics.GetPlayerCharacter` 0)))
  (bind _output_get (set `self.Player Ref` _asbp_lucid_driver))
  (`|AIMoveTo` self (`self.Player POS`) _output_get))

(event `Get Player Position`
  (set `self.Player POS` (`self.K2_GetActorLocation` (`self.Player Ref`))))

(event `PerformAttack`
  (bind _attackmontages (`self.AttackMontages`))
  (`AnimInstance.Montage_Play` (`SkeletalMeshComponent.GetAnimInstance` (`self.Mesh`)) (`|GetArrayItem` _attackmontages (`KismetMathLibrary.RandomIntegerInRange` 0 (`KismetArrayLibrary.Array_Length` _attackmontages))) 1.0 "MontageLength" 0.0 true))

(event `self.AttackRange.OnComponentBeginOverlap`
  (params (OverlappedComponent :type "PrimitiveComponent Object Reference") (OtherActor :type "Actor Object Reference") (OtherComp :type "PrimitiveComponent Object Reference") (OtherBodyIndex :type Integer) (bFromSweep :type Boolean) (SweepResult :type "HitResult Structure (by ref)"))
  (cast `/Game/-Blueprints/Character/BP_LucidDriver` OtherActor)
  (bind _output_get (set `self.IsInRange` true))
  (`MovementComponent.StopMovementImmediately` (`self.CharacterMovement`)))

(event `self.AttackRange.OnComponentEndOverlap`
  (params (OverlappedComponent :type "PrimitiveComponent Object Reference") (OtherActor :type "Actor Object Reference") (OtherComp :type "PrimitiveComponent Object Reference") (OtherBodyIndex :type Integer)))

(fn `UserConstructionScript`)